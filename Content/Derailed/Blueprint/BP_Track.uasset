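; BP_Track is a repairable track piece that tracks a Damage value.
; Its Box overlap sets InRange on the TopDownCharacter as it enters and leaves.
; The Interaction event adds AmountToRepair to Damage, which behaves like health.
; Tick polls that value and uses DoOnce gates to print Destroyed at zero or below, or otherwise check once whether to print Fixed.
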(event OnComponentBeginOverlap(Box)
  (params (OverlappedComponent :type Primitive%20Component%20Object%20Reference) (OtherActor :type Actor%20Object%20Reference) (OtherComp :type Primitive%20Component%20Object%20Reference) (OtherBodyIndex :type Integer) (bFromSweep :type Boolean) (SweepResult :type Hit%20Result%20Structure%20%28by%20ref%29))
  (bind _astop_down_character (Utilities|Casting|CastToTopDownCharacter OtherActor))
  (Variables|/Game/TopDownBP/Blueprints/TopDownCharacter.TopDownCharacter_C|SetInRange _astop_down_character true))

(event OnComponentEndOverlap(Box)
  (params (OverlappedComponent :type Primitive%20Component%20Object%20Reference) (OtherActor :type Actor%20Object%20Reference) (OtherComp :type Primitive%20Component%20Object%20Reference) (OtherBodyIndex :type Integer))
  (bind _astop_down_character (Utilities|Casting|CastToTopDownCharacter OtherActor))
  (Variables|/Game/TopDownBP/Blueprints/TopDownCharacter.TopDownCharacter_C|SetInRange _astop_down_character false))

(event EventTick
  (params (DeltaSeconds :type Float%20%28single-precision%29))
  (if (<= (Variables|Default|GetDamage) 0)
    (Utilities|FlowControl|DoOnce false
      (:Completed
        (Development|PrintString "Destroyed")))
    (else
      (Utilities|FlowControl|DoOnce false
        (:Completed
          (if (>= (Variables|Default|GetDamage) (Variables|Default|GetAmountToRepair))
            (Development|PrintString "Fixed")))))))

(event EventInteraction
  (params (ActorHit :type Actor%20Object%20Reference))
  (Variables|Default|SetDamage (+ (Variables|Default|GetDamage) (Variables|Default|GetAmountToRepair))))

(fn ConstructionScript)