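; Long track segment that breaks down over time, can be repaired by interaction, and crashes trains that hit it while broken.
; Damage works as track health: Interaction raises it, and Tick swaps three meshes between broken and intact at the thresholds.
; A random delay loop, started by Tick or overlap, zeroes it unless TrainNearby is set.
; A Train-tagged actor overlapping Box on broken track triggers an explosion sound and CrashMessage.
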(event OnComponentBeginOverlap(Box)
  (params (OverlappedComponent :type Primitive%20Component%20Object%20Reference) (OtherActor :type Actor%20Object%20Reference) (OtherComp :type Primitive%20Component%20Object%20Reference) (OtherBodyIndex :type Integer) (bFromSweep :type Boolean) (SweepResult :type Hit%20Result%20Structure%20%28by%20ref%29))
  ;[1 1 1] Makes the train crash
  (Utilities|FlowControl|Sequence
    (:then_0
      (if (and (Actor|ActorHasTag OtherActor "Train") (<= (Variables|Default|GetDamage) 0))
        (Audio|PlaySoundatLocation "/Game/Derailed/Sound/Train_Explosion_v_1.Train_Explosion_v_1" (Transformation|GetActorLocation) "0, 0, 0" 1.0 1.0 0.0 0 0 0)
        (Class|BPICrash|Crash(Message) OtherActor)))
    (:then_1
      (Utilities|FlowControl|RetriggerableDelay (Math|Conversions|ToFloat(Integer) (Math|Random|RandomIntegerinRange 25 30)))
      (if (not (Variables|Default|GetTrainNearby))
        (Variables|Default|SetDamage 0)
        (Utilities|FlowControl|DoOnce false) ; enters at Reset
      ))))

(event EventTick
  (params (DeltaSeconds :type Float%20%28single-precision%29))
  ;[1 1 1] Sets the mesh when track is damaged
  (Utilities|FlowControl|Sequence
    (:then_0
      (if (<= (Variables|Default|GetDamage) 0)
        (Components|StaticMesh|SetStaticMesh (Variables|Default|GetTracks) "/Game/Derailed/Meshes/SM_BrokenTracks.SM_BrokenTracks")
        (Components|StaticMesh|SetStaticMesh (Variables|Default|GetTracks1) "/Game/Derailed/Meshes/SM_BrokenTracks.SM_BrokenTracks")
        (Components|StaticMesh|SetStaticMesh (Variables|Default|GetTracks2) "/Game/Derailed/Meshes/SM_BrokenTracks.SM_BrokenTracks")
        (elif (>= (Variables|Default|GetDamage) 100)
          (Components|StaticMesh|SetStaticMesh (Variables|Default|GetTracks) "/Game/Derailed/Meshes/SM_tracks.SM_Tracks")
          (Components|StaticMesh|SetStaticMesh (Variables|Default|GetTracks1) "/Game/Derailed/Meshes/SM_tracks.SM_Tracks")
          (Components|StaticMesh|SetStaticMesh (Variables|Default|GetTracks2) "/Game/Derailed/Meshes/SM_tracks.SM_Tracks"))))
    (:then_1
      (Utilities|FlowControl|DoOnce false :!label _label
        (:Completed
          (Utilities|FlowControl|RetriggerableDelay (Math|Conversions|ToFloat(Integer) (Math|Random|RandomIntegerinRange 25 30)))
          (if (not (Variables|Default|GetTrainNearby))
            (Variables|Default|SetDamage 0)
            (goto _label Reset)))))))

(event EventInteraction
  (params (ActorHit :type Actor%20Object%20Reference))
  ;[1 1 1] Repairing the track
  (Variables|Default|SetDamage (+ (Variables|Default|GetDamage) 10)))

(fn ConstructionScript)