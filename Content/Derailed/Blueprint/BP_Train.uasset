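; BP_Train is a train actor in Derailed that starts moving along the Y axis as soon as it spawns.
; The Movement timeline adds its TrainMovement value to the current Y every update, via a Lerp fixed at full alpha.
; A spawn sound plays at start and a loop sound follows after a delay.
; Its Crash event increments the TopDownCharacter player's crash count and destroys the train.
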(event EventBeginPlay
  (bind _returnvalue (Transformation|GetActorLocation))
  (bind _returnvalue_2 (Transformation|GetActorLocation))
  (bind (_x _y _z) (Math|Vector|BreakVector _returnvalue))
  (Utilities|FlowControl|Sequence
    (:then_0
      (bind _trainmovement (Timeline|Movement Play)
        (:Update
          (Transformation|SetActorRelativeLocation (Math|Vector|MakeVector _x (Math|Float|Lerp _y (+ _trainmovement _y) 1.0) _z)))))
    (:then_1
      (Audio|PlaySoundatLocation "/Game/Derailed/Sound/Train_Spawn.Train_Spawn" _returnvalue_2 "0, 0, 0" 0.3 1.0 0.0 0 0 0)
      (Utilities|FlowControl|Delay 4.0)
      (Audio|PlaySoundatLocation "/Game/Derailed/Sound/Train_Loop.Train_Loop" _returnvalue_2 "0, 0, 0" 1.0 1.0 0.0 0 0 0))))

(event EventCrash
  (bind _astop_down_character (Utilities|Casting|CastToTopDownCharacter (Game|GetPlayerCharacter 0)))
  (Default|IncreaseCrashes _astop_down_character)
  (Actor|DestroyActor))

(fn ConstructionScript)